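; Speed boost pad that multiplies the linear velocity of any WheeledVehicle entering its Box trigger.
; On overlap it stores the mesh's velocity in CurrentVelocity and applies a scaled-up copy to the movement component's updated primitive.
; After exit and a delay, it lerps toward the stored velocity, but the zero alpha leaves the current velocity unchanged.
; The IsAI function only stores StaticMesh's velocity, with no AI check.
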(event OnComponentBeginOverlap(Box)
  (params (OtherActor :type Actor%20Object%20Reference) (OtherComp :type Primitive%20Component%20Object%20Reference) (OtherBodyIndex :type Integer) (bFromSweep :type Boolean) (SweepResult :type Hit%20Result%20Structure%20%28by%20ref%29))
  (bind _aswheeled_vehicle (Utilities|Casting|CastToWheeledVehicle OtherActor))
  (bind _returnvalue (Physics|GetPhysicsLinearVelocity (Variables|/Script/Engine.WheeledVehicle|GetMesh _aswheeled_vehicle) "None"))
  (bind _output_get (Variables|Default|SetCurrentVelocity _returnvalue))
  (Physics|SetPhysicsLinearVelocity (Variables|/Script/Engine.MovementComponent|GetUpdatedPrimitive (Variables|/Script/Engine.WheeledVehicle|GetVehicleMovement _aswheeled_vehicle)) (* _output_get 1.5) false "None"))

(event OnComponentEndOverlap(Box)
  (params (OtherActor :type Actor%20Object%20Reference) (OtherComp :type Primitive%20Component%20Object%20Reference) (OtherBodyIndex :type Integer))
  (bind _aswheeled_vehicle (Utilities|Casting|CastToWheeledVehicle OtherActor))
  (Utilities|FlowControl|Delay 2.0)
  (bind _returnvalue (Physics|GetPhysicsLinearVelocity (Variables|/Script/Engine.MovementComponent|GetUpdatedPrimitive (Variables|/Script/Engine.WheeledVehicle|GetVehicleMovement _aswheeled_vehicle)) "None"))
  (Physics|SetPhysicsLinearVelocity (Variables|/Script/Engine.MovementComponent|GetUpdatedPrimitive (Variables|/Script/Engine.WheeledVehicle|GetVehicleMovement _aswheeled_vehicle)) (Math|Vector|Lerp(Vector) _returnvalue (Variables|Default|GetCurrentVelocity) 0.0) false "None"))

(event EventBeginPlay)

(event EventTick
  (params (DeltaSeconds :type Float%20%28single-precision%29)))

(fn ConstructionScript)

(fn IsAI?
  (bind _returnvalue (Physics|GetPhysicsLinearVelocity (Variables|Default|GetStaticMesh) "None"))
  (Variables|Default|SetCurrentVelocity _returnvalue))