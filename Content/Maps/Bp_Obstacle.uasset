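; Bp_Obstacle is an obstacle actor that slows wheeled vehicles that overlap its box.
; On overlap it stores the vehicle mesh's linear velocity and sets the movement component's updated primitive to a quarter of it.
; After a delay it sets velocity again through a lerp toward the stored value, but the zero alpha keeps the current velocity, so the original speed is not restored.
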(event OnComponentBeginOverlap(Box)
  (params (OtherActor :type Actor%20Object%20Reference) (OtherComp :type Primitive%20Component%20Object%20Reference) (OtherBodyIndex :type Integer) (bFromSweep :type Boolean) (SweepResult :type Hit%20Result%20Structure%20%28by%20ref%29))
  (bind _aswheeled_vehicle (Utilities|Casting|CastToWheeledVehicle OtherActor))
  (bind _returnvalue (Physics|GetPhysicsLinearVelocity (Variables|/Script/Engine.WheeledVehicle|GetMesh _aswheeled_vehicle) "None"))
  (bind _output_get (Variables|Default|SetCurretVelocity _returnvalue))
  (Physics|SetPhysicsLinearVelocity (Variables|/Script/Engine.MovementComponent|GetUpdatedPrimitive (Variables|/Script/Engine.WheeledVehicle|GetVehicleMovement _aswheeled_vehicle)) (/ _output_get 4.0) false "None")
  (Utilities|FlowControl|Delay 4.0)
  (bind _returnvalue_2 (Physics|GetPhysicsLinearVelocity (Variables|/Script/Engine.MovementComponent|GetUpdatedPrimitive (Variables|/Script/Engine.WheeledVehicle|GetVehicleMovement _aswheeled_vehicle)) "None"))
  (Physics|SetPhysicsLinearVelocity (Variables|/Script/Engine.MovementComponent|GetUpdatedPrimitive (Variables|/Script/Engine.WheeledVehicle|GetVehicleMovement _aswheeled_vehicle)) (Math|Vector|Lerp(Vector) _returnvalue_2 (Variables|Default|GetCurretVelocity) 0.0) false "None"))

(event EventBeginPlay)

(event EventActorBeginOverlap
  (params (OtherActor :type Actor%20Object%20Reference)))

(event EventTick
  (params (DeltaSeconds :type Float%20%28single-precision%29)))

(fn ConstructionScript)