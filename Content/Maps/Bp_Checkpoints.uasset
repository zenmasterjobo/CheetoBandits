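; Checkpoint Blueprint with a trigger volume, particle effect and arrow marking its forward direction.
; When the player pawn exits the trigger, a dot product of its velocity and the arrow's forward vector confirms it is moving the correct way.
; On success it calls CheckpointCleared with its checkpoint number, then hides trigger and particles and disables further overlap events.
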(event OnComponentEndOverlap(Trigger)
  (params (OtherActor :type Actor%20Object%20Reference) (OtherComp :type Primitive%20Component%20Object%20Reference) (OtherBodyIndex :type Integer))
  (bind _trigger (Variables|Default|GetTrigger))
  (bind _asmy_project_3pawn (Utilities|Casting|CastToMyProject3Pawn OtherActor))
  (if (> (Math|Vector|DotProduct (Transformation|GetVelocity _asmy_project_3pawn) (Math|Rotator|GetRotationXVector (Transformation|GetWorldRotation (Variables|Default|GetArrow)))) 0.0)
    (Default|CallCheckpointCleared (Variables|Default|GetCheckpointNumber))
    (Development|SetHiddeninGame _trigger true false)
    (Variables|/Script/Engine.PrimitiveComponent|SetbGenerateOverlapEvents _trigger false)))

(event EventBeginPlay)

(event EventActorBeginOverlap
  (params (OtherActor :type Actor%20Object%20Reference)))

(event EventTick
  (params (DeltaSeconds :type Float%20%28single-precision%29)))

(fn ConstructionScript)