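; Checkpoint actor that registers when a vehicle passes through it in the intended direction.
; When a Bp_Vehicle leaves the trigger, a dot product of its velocity with the Arrow component's forward vector rejects wrong-way exits.
; A valid pass broadcasts CheckpointCleared with the checkpoint number, hides the trigger and particle system, and disables the trigger's overlap events so it does not fire again.
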(event OnComponentEndOverlap(Trigger)
  (params (OtherActor :type Actor%20Object%20Reference) (OtherComp :type Primitive%20Component%20Object%20Reference) (OtherBodyIndex :type Integer))
  (bind _trigger (Variables|Default|GetTrigger))
  ;[1 1 1] Checkpoint - clear when overlap
  (bind _asbp_vehicle (Utilities|Casting|CastToBp_Vehicle OtherActor))
  (if (> (Math|Vector|DotProduct (Transformation|GetVelocity _asbp_vehicle) (Math|Rotator|GetRotationXVector (Transformation|GetWorldRotation (Variables|Default|GetArrow)))) 0.0)
    (Default|CallCheckpointCleared (Variables|Default|GetCheckpointNumber))
    (Development|SetHiddeninGame _trigger true false)
    (Variables|/Script/Engine.PrimitiveComponent|SetbGenerateOverlapEvents _trigger false)))

(event EventBeginPlay)

(event EventActorBeginOverlap
  (params (OtherActor :type Actor%20Object%20Reference)))

(event EventTick
  (params (DeltaSeconds :type Float%20%28single-precision%29)))

(fn ConstructionScript)