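; HUD Blueprint that draws the driven vehicle's speed in km/h and current gear, with N for neutral and a red R for reverse.
; DrawHUD scales text position and size from a 1280x720 reference.
; MyGame's Swap flag picks the data source: the owning Sedan's or the AiPawn's vehicle movement.
; A separate Timer function draws minutes and seconds at unscaled coordinates but is not called in this Blueprint.
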(event EventDrawHUD
  (params (SizeX :type Integer) (SizeY :type Integer))
  ;[1 1 1] Calculate ratio from 720p
  (Utilities|FlowControl|Sequence
    (:then_0
      (bind _asmy_game (Utilities|Casting|CastToMyGame (Game|GetGameMode))))
    (:then_1
      (Variables|Default|SetHUDXRatio (/ (Math|Conversions|ToFloat(Integer) SizeX) 1.28e+03)))
    (:then_2
      (Variables|Default|SetHUDYRatio (/ (Math|Conversions|ToFloat(Integer) SizeY) 7.2e+02)))
    (:then_3
      ;[1 1 1] Get Vehicle Movement component
      (bind _assedan (Utilities|Casting|CastToSedan (Class|HUD|GetOwningPawn)))
      ;[1 1 1] Print vehicle speed
      (HUD|DrawText (Utilities|String|Append (Utilities|String|ToString(Integer) (Math|Float|Floor (Math|Float|Absolute(Float) (* (Vehicle|GetForwardSpeed (Utilities|Select :Index (Math|Conversions|ToInteger(Boolean) (Variables|/Game/Blueprints/MyGame.MyGame_C|Getswap _asmy_game)) :Option%200 (Variables|/Script/Engine.WheeledVehicle|GetVehicleMovement _assedan) :Option%201 (Variables|/Script/Engine.WheeledVehicle|GetVehicleMovement (Variables|/Game/Blueprints/MyGame.MyGame_C|GetaiPawn _asmy_game)))) 0.036)))) " km/h") "(R=1.000000,G=1.000000,B=1.000000,A=1.000000)" (* 805.0 (Variables|Default|GetHUDXRatio)) (* 455.0 (Variables|Default|GetHUDYRatio)) "/Engine/EngineFonts/RobotoDistanceField.RobotoDistanceField" (* 1.4 (Variables|Default|GetHUDYRatio)) false)
      ;[1 1 1] Print vehicle gear
      (if (> (Class|WheeledVehicleMovementComponent|GetCurrentGear (Utilities|Select :Index (Math|Conversions|ToInteger(Boolean) (Variables|/Game/Blueprints/MyGame.MyGame_C|Getswap _asmy_game)) :Option%200 (Variables|/Script/Engine.WheeledVehicle|GetVehicleMovement _assedan) :Option%201 (Variables|/Script/Engine.WheeledVehicle|GetVehicleMovement (Variables|/Game/Blueprints/MyGame.MyGame_C|GetaiPawn _asmy_game)))) -1)
        (HUD|DrawText (Utilities|String|Append "Gear: " (select (== (Class|WheeledVehicleMovementComponent|GetCurrentGear (Utilities|Select :Index (Math|Conversions|ToInteger(Boolean) (Variables|/Game/Blueprints/MyGame.MyGame_C|Getswap _asmy_game)) :Option%200 (Variables|/Script/Engine.WheeledVehicle|GetVehicleMovement _assedan) :Option%201 (Variables|/Script/Engine.WheeledVehicle|GetVehicleMovement (Variables|/Game/Blueprints/MyGame.MyGame_C|GetaiPawn _asmy_game)))) 0) "N" (Utilities|String|ToString(Integer) (Class|WheeledVehicleMovementComponent|GetCurrentGear (Utilities|Select :Index (Math|Conversions|ToInteger(Boolean) (Variables|/Game/Blueprints/MyGame.MyGame_C|Getswap _asmy_game)) :Option%200 (Variables|/Script/Engine.WheeledVehicle|GetVehicleMovement _assedan) :Option%201 (Variables|/Script/Engine.WheeledVehicle|GetVehicleMovement (Variables|/Game/Blueprints/MyGame.MyGame_C|GetaiPawn _asmy_game))))))) "(R=1.000000,G=1.000000,B=1.000000,A=1.000000)" (* 805.0 (Variables|Default|GetHUDXRatio)) (* 5e+02 (Variables|Default|GetHUDYRatio)) "/Engine/EngineFonts/RobotoDistanceField.RobotoDistanceField" (* 1.4 (Variables|Default|GetHUDYRatio)) false) ; If True display Current Gear
        (else
          (HUD|DrawText "Gear: R" "(R=1.000000,G=0.000000,B=0.000000,A=1.000000)" (* 805.0 (Variables|Default|GetHUDXRatio)) (* 5e+02 (Variables|Default|GetHUDYRatio)) "/Engine/EngineFonts/RobotoDistanceField.RobotoDistanceField" (* 1.4 (Variables|Default|GetHUDYRatio)) false) ; If False display R for Reverse
        )))))

(fn ConstructionScript)

(fn Timer
  (if (> 9 (Variables|Default|GetHud_Time_Second))
    (HUD|DrawText (Utilities|String|ToString(Text) (Utilities|Text|ToText(String) (Utilities|String|Append (Utilities|String|Append (Utilities|String|ToString(Integer) (Variables|Default|GetHud_Time_Minute)) ":") (Utilities|String|ToString(Integer) (Variables|Default|GetHud_Time_Second))))) "(R=1.000000,G=1.000000,B=1.000000,A=1.000000)" 9e+02 5e+02 "/Game/Fonts/Time.Time" 1.0 false)
    (else
      (HUD|DrawText (Utilities|String|ToString(Text) (Utilities|Text|ToText(String) (Utilities|String|Append (Utilities|String|Append (Utilities|String|ToString(Integer) (Variables|Default|GetHud_Time_Minute)) ":0") (Utilities|String|ToString(Integer) (Variables|Default|GetHud_Time_Second))))) "(R=1.000000,G=1.000000,B=1.000000,A=1.000000)" 9e+02 5e+02 "/Game/Fonts/Time.Time" 1.0 false))))