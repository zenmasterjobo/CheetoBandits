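; Race manager actor that tracks checkpoints, laps and a countdown timer for the player's vehicle.
; On BeginPlay it copies race settings and target times to Bp_PlayerController, numbers the checkpoints and starts a reversed timeline as the on-screen countdown.
; Each cleared checkpoint activates the next, updates the respawn transform and resets the timer, with laps checked on wrap-around.
; Timeout or race completion stops the car and triggers a restart.
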(event Custom|ApplySettings
  (bind _controllerreference (Variables|Default|GetControllerReference))
  ;[1 1 1] Apply Settings at the beginning of the play.
  (Variables|/Game/Blueprints/Bp_PlayerController.Bp_PlayerController_C|SetMaxLaps _controllerreference (Variables|CustomSettings|GetMaxLaps))
  (Variables|/Game/Blueprints/Bp_PlayerController.Bp_PlayerController_C|SetSaveSlot _controllerreference (Variables|CustomSettings|GetSaveGameName))
  (Variables|/Game/Blueprints/Bp_PlayerController.Bp_PlayerController_C|SetNameOfMap _controllerreference (Variables|CustomSettings|GetNameOfMap))
  (CallFunction|UpdateTimes)
  (Default|StartGameSetup _controllerreference))

(event Custom|StartSequence
  ;[1 1 1] Starting sequence for the checkpoints.
  (for (_array_element _array_index) (Variables|Checkpoints|GetCheckpoints)
    (Variables|/Game/Blueprints/Bp_Checkpoints.Bp_Checkpoints_C|SetCheckpointNumber _array_element (+ _array_index 1))
    (CallFunction|ActivateCheckpoint (Utilities|Array|Get(acopy) (Variables|Checkpoints|GetCheckpoints)))
    (for _array_element_2 (Variables|Checkpoints|GetCheckpoints)
      (EventDispatchers|AssignCheckpointCleared _array_element_2 (delegate Custom|Checkpoint%20Cleared)))))

(event Custom|Checkpoint%20Cleared
  (params (NextCheckpoint :type Integer))
  (bind _controllerreference (Variables|Default|GetControllerReference))
  ;[1 1 1] Checkpoint cleared - also check for race end
  (CallFunction|LapCheck NextCheckpoint)
  (Audio|Components|Audio|Play (Variables|/Script/Engine.AmbientSound|GetAudioComponent (Variables|CustomSettings|GetCheckpointSoundFX)) 0.0)
  (if (Variables|/Game/Blueprints/Bp_PlayerController.Bp_PlayerController_C|GetRaceComplete _controllerreference)
    (Default|Restart _controllerreference)
    (else
      (bind _gametime (Timeline|TimeLine SetNewTime)
        (:Update
          ;[1 1 1] Print Time to the Screen
          (bind _output_get (Variables|CustomSettings|SetActualRaceTime _gametime))
          (bind _output_get_2 (Variables|CustomSettings|SetCheckpointTextCountdown (Utilities|TimetoText _output_get)))
          (Development|PrintText _output_get_2))
        (:Finished
          ;[1 1 1] Handle restarting the game wen the time rruns out
          (Development|PrintText "OUT OF TIME!")
          (bind _aswheeled_vehicle (Utilities|Casting|CastToWheeledVehicle (Game|Player|GetPlayerPawn 0)))
          (Class|WheeledVehicleMovementComponent|SetHandbrakeInput (Variables|/Script/Engine.WheeledVehicle|GetVehicleMovement _aswheeled_vehicle) true)
          (Input|DisableInput _aswheeled_vehicle (Variables|Default|GetControllerReference))
          (Utilities|FlowControl|Delay 4.0)
          (Development|ExecuteConsoleCommand "RestartLevel"))))))

(event EventBeginPlay)

(event EventActorBeginOverlap
  (params (OtherActor :type Actor%20Object%20Reference)))

(event EventTick
  (params (DeltaSeconds :type Float%20%28single-precision%29)))

(event EventBeginPlay
  ;[1 1 1] Begin Play
  (bind _asbp_player_controller (Utilities|Casting|CastToBp_PlayerController (Game|GetPlayerController 0)))
  (Variables|Default|SetControllerReference _asbp_player_controller)
  (CallFunction|ApplySettings)
  (CallFunction|StartSequence)
  (bind _gametime (Timeline|TimeLine ReverseFromEnd)
    (:Update
      ;[1 1 1] Print Time to the Screen
      (bind _output_get (Variables|CustomSettings|SetActualRaceTime _gametime))
      (bind _output_get_2 (Variables|CustomSettings|SetCheckpointTextCountdown (Utilities|TimetoText _output_get)))
      (Development|PrintText _output_get_2))
    (:Finished
      ;[1 1 1] Handle restarting the game wen the time rruns out
      (Development|PrintText "OUT OF TIME!")
      (bind _aswheeled_vehicle (Utilities|Casting|CastToWheeledVehicle (Game|Player|GetPlayerPawn 0)))
      (Class|WheeledVehicleMovementComponent|SetHandbrakeInput (Variables|/Script/Engine.WheeledVehicle|GetVehicleMovement _aswheeled_vehicle) true)
      (Input|DisableInput _aswheeled_vehicle (Variables|Default|GetControllerReference))
      (Utilities|FlowControl|Delay 4.0)
      (Development|ExecuteConsoleCommand "RestartLevel"))))

(fn ConstructionScript)

(fn UpdateTimes
  (bind _controllerreference (Variables|Default|GetControllerReference))
  ;[1 1 1] User times
  (Variables|/Game/Blueprints/Bp_PlayerController.Bp_PlayerController_C|SetGoldTime _controllerreference (Variables|CustomSettings|GetGoldTime))
  (Variables|/Game/Blueprints/Bp_PlayerController.Bp_PlayerController_C|SetSilverTime _controllerreference (Variables|CustomSettings|GetSilverTime))
  (Variables|/Game/Blueprints/Bp_PlayerController.Bp_PlayerController_C|SetBronzeTime _controllerreference (Variables|CustomSettings|GetBronzeTime))
  (Variables|/Game/Blueprints/Bp_PlayerController.Bp_PlayerController_C|SetDefaultBestLapTime _controllerreference (Variables|CustomSettings|GetDefaultBestLap))
  (Variables|/Game/Blueprints/Bp_PlayerController.Bp_PlayerController_C|SetDefaultBestRaceTime _controllerreference (Variables|CustomSettings|GetDefaultBestTime)))

(fn LapCheck
  (params (Checkpoint :type Integer))
  ;[1 1 1] Lap check
  (bind _output_get (LocalVariables|SetLocalCheckpoint Checkpoint))
  (if (== _output_get 0)
    (bind _isracecomplete (CallFunction|RaceCompleteCheck))
    (if _isracecomplete
      _
      (else
        (CallFunction|ActivateCheckpoint (Utilities|Array|Get(acopy) (Variables|Checkpoints|GetCheckpoints)))))
    (Default|UpdateLap (Variables|Default|GetControllerReference))
    (else
      (CallFunction|ActivateCheckpoint (Utilities|Array|Get(acopy) (Variables|Checkpoints|GetCheckpoints) (LocalVariables|GetLocalCheckpoint)))))
  (Variables|/Game/Blueprints/Bp_PlayerController.Bp_PlayerController_C|SetRespawnLocation (Variables|Default|GetControllerReference) (Math|Transform|MakeTransform (+ (.Location (Math|Transform|BreakTransform (Transformation|GetActorTransform (Utilities|Array|Get(acopy) (Variables|Checkpoints|GetCheckpoints) (- (LocalVariables|GetLocalCheckpoint) 1))))) "0, 0,128.000000") (.Rotation (Math|Transform|BreakTransform (Transformation|GetActorTransform (Utilities|Array|Get(acopy) (Variables|Checkpoints|GetCheckpoints) (- (LocalVariables|GetLocalCheckpoint) 1))))))))

(fn ActivateCheckpoint
  (params (NextCheckpoint :type Bp%20Checkpoints%20Object%20Reference))
  (bind _trigger (Variables|/Game/Blueprints/Bp_Checkpoints.Bp_Checkpoints_C|GetTrigger NextCheckpoint))
  ;[1 1 1] This activates the checkpoints
  (Development|SetHiddeninGame _trigger false false)
  (Variables|/Script/Engine.PrimitiveComponent|SetbGenerateOverlapEvents _trigger true))

(fn RaceCompleteCheck
  (bind _controllerreference (Variables|Default|GetControllerReference))
  (bind _controllerreference_2 (Variables|Default|GetControllerReference))
  (if (>= (Variables|/Game/Blueprints/Bp_PlayerController.Bp_PlayerController_C|GetActualLap _controllerreference) (Variables|/Game/Blueprints/Bp_PlayerController.Bp_PlayerController_C|GetMaxLaps _controllerreference))
    (bind _output_get (Variables|/Game/Blueprints/Bp_PlayerController.Bp_PlayerController_C|SetRaceComplete _controllerreference_2 true))
    (LocalVariables|SetLocalComplete _output_get)
    (bind _aswheeled_vehicle (Utilities|Casting|CastToWheeledVehicle (Game|Player|GetPlayerPawn 0)))
    (Class|WheeledVehicleMovementComponent|SetHandbrakeInput (Variables|/Script/Engine.WheeledVehicle|GetVehicleMovement _aswheeled_vehicle) true)
    (Input|DisableInput _aswheeled_vehicle (Variables|Default|GetControllerReference))
    (Components|Activation|Deactivate (Variables|/Script/Engine.WheeledVehicle|GetMesh _aswheeled_vehicle))
    (else
      (bind _output_get_2 (Variables|/Game/Blueprints/Bp_PlayerController.Bp_PlayerController_C|SetRaceComplete _controllerreference_2 false))
      (LocalVariables|SetLocalComplete _output_get_2)))
  (return (LocalVariables|GetLocalComplete)))